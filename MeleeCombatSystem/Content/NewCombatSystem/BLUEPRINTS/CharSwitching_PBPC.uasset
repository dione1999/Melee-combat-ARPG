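; Player controller that lets the player switch control between the NCC_Char_BP characters in the level by pressing Tab.
; On BeginPlay it gathers all NCC_Char_BP actors into a list and records the player's character as the current one.
; Each Tab press runs NewFunction, which finds the current character's index, advances to the next one, wrapping to the first at the end, and possesses it.
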(event EventBeginPlay
  (bind _outactors (Actor|GetAllActorsOfClass "/Game/NewCombatSystem/BLUEPRINTS/NCC_Char_BP.NCC_Char_BP_C"))
  (Variables|Default|SetChar%20List _outactors)
  (bind _asncc_char_bp (Utilities|Casting|CastToNCC_Char_BP (Game|GetPlayerCharacter 0)))
  (Variables|Default|SetCunnernt%20Char _asncc_char_bp))

(event EventTick
  (params (DeltaSeconds :type Float%20%28single-precision%29)))

(event Input|KeyboardEvents|Tab
  (params (Key :type Key%20Structure))
  (:Pressed
    (CallFunction|NewFunction)))

(fn ConstructionScript)

(fn NewFunction
  (LocalVariables|Setlocal%20index (Utilities|Array|FindItem (Variables|Default|GetChar%20List) (Variables|Default|GetCunnernt%20Char)))
  (bind _output_get (LocalVariables|Setlocal%20index (Math|Integer|SelectInt (+ (Utilities|Array|FindItem (Variables|Default|GetChar%20List) (Variables|Default|GetCunnernt%20Char)) 1) 0 (Utilities|Array|IsValidIndex (Variables|Default|GetChar%20List) (+ (Utilities|Array|FindItem (Variables|Default|GetChar%20List) (Variables|Default|GetCunnernt%20Char)) 1)))))
  (bind _output_get_2 (Variables|Default|SetCunnernt%20Char (Utilities|Array|Get(acopy) (Variables|Default|GetChar%20List) _output_get)))
  (Pawn|Possess _output_get_2))