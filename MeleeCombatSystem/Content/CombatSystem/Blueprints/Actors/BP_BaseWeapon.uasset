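; Base weapon actor that registers as the owner's main weapon when equipped, sets its combat type on the anim instance and supplies montages per action gameplay tag.
; A collision component, toggled on demand, reports hits, which deal point damage to actors that can receive it.
; Damage multipliers and stat costs are looked up from the owner's current state-manager action.
; It also drives socket-based trail and dust effects and can switch to physics simulation.
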(event OnHit(BP_MainCollisionComponent)
  (params (HitResult :type Hit%20Result%20Structure))
  (CallFunction|OnHit HitResult))

(event Custom|SimulateWeaponPhysics
  (Collision|SetCollisionProfileName (CallFunction|GetItemMesh) "PhysicsActor" true :!class /Script/Engine.PrimitiveComponent)
  (Physics|SetSimulatePhysics (CallFunction|GetItemMesh) true))

(event Custom|ToggleCombat
  (params (bEnableCombat? :type Boolean))
  (Default|SetCombatEnable (Variables|Default|GetBP_CombatComponent) bEnableCombat?))

(event EventBeginPlay
  (|CallParentFunction)
  (Effects|Components|ParticleSystem|SetTemplate (Variables|Default|GetParticleSystem_Trail) (Variables|FX|GetTrailFX))
  (Components|Activation|Deactivate (Variables|Default|GetParticleSystem_Trail)))

(event Collision|EventActorBeginOverlap
  (params (OtherActor :type Actor%20Object%20Reference))
  (|CallParentFunction OtherActor) ; This node is disabled and will not be called.\nDrag off pins to build functionality.
)

(event EventTick
  (params (DeltaSeconds :type Float%20%28single-precision%29))
  (|CallParentFunction DeltaSeconds) ; This node is disabled and will not be called.\nDrag off pins to build functionality.
)

(fn ConstructionScript
  (|CallParentFunction))

(fn OnEquipped
  (|CallParentFunction)
  (Variables|Default|SetBP_CombatComponent (Actor|GetComponentbyClass (Components|GetOwner) "/Game/CombatSystem/Blueprints/Components/BP_CombatComponent.BP_CombatComponent_C"))
  (Variables|Default|SetBP_StateManagerComponent (Actor|GetComponentbyClass (Components|GetOwner) "/Game/CombatSystem/Blueprints/Components/BP_StateManagerComponent.BP_StateManagerComponent_C"))
  (Default|SetMainWeapon (Variables|Default|GetBP_CombatComponent) self)
  (Class|AnimInstanceBPI|UpdateCombatType(Message) (Components|SkeletalMesh|GetAnimInstance (Variables|/Script/Engine.Character|GetMesh (.AsCharacter (Utilities|Casting|CastToCharacter (Components|GetOwner))))) (Variables|Initialization|GetCombatType))
  (Default|SetCollisionMeshComponent (Variables|Default|GetBP_MainCollisionComponent) (Variables|Default|GetItemStaticMesh))
  (Default|AddIgnoreActor (Variables|Default|GetBP_MainCollisionComponent) (Components|GetOwner)))

(fn OnHit
  (params (Hit :type Hit%20Result%20Structure%20%28by%20ref%29))
  (bind _hitactor (Collision|BreakHitResult Hit))
  (bind _returnvalue (Class|CombatBPI|CanRecieveDamage(Message) _hitactor))
  (if _returnvalue
    (Game|Damage|ApplyPointDamage _hitactor (Stats|GetDamage) (Transformation|GetActorForwardVector (Components|GetOwner)) Hit (Game|GetInstigatorController) self (Variables|Initialization|GetDamage%20Type%20Class))))

(fn GetActionMontages
  (params (CharacterAction :type Gameplay%20Tag%20Structure))
  (|SwitchGameplayTag CharacterAction
    (:Character.Action.Attack.Light%20Attack
      (return (Variables|Animations|GetLightAttackMontages)))
    (:Character.Action.Attack.Heavy%20Attack
      (return (Variables|Animations|GetHeavyAttackMontages)))
    (:Character.Action.Attack.Charged%20Attack
      (return (Variables|Animations|GetChargedAttackMontages)))
    (:Character.Action.Attack.Falling%20Attack
      (return (Variables|Animations|GetFallingAttackMontages)))
    (:Character.Action.Attack.Sprinting%20Attack
      (return (Variables|Animations|GetSprintingAttackMontages)))
    (:Character.Action.Dodge
      (return (Variables|Animations|GetDodgeMontages)))
    (:Character.Action.Die
      (return (Variables|Animations|GetDieMontages)))
    (:Character.Action.Enter%20Combat
      (return (Utilities|Array|MakeArray (Variables|Animations|GetEnterCombat))))
    (:Character.Action.Exit%20Combat
      (return (Utilities|Array|MakeArray (Variables|Animations|GetExitCombat))))
    (:Character.Action.Attack.Special%20Attack
      (return (Variables|Animations|GetSpecialAttackMontages)))
    (:Character.Action.Slide
      (return (Variables|Animations|GetSlideMontages)))
    (:Character.Action.Attack.Stealth%20Attack
      (return 0))
    (:Character.Action.Waiting%20For%20Executed
      (return (Variables|Animations|GetWaitForExecutedMontages)))
    (:Character.Action.Executed
      (return (Variables|Animations|GetExecutedMontages)))
    (:Character.Action.Execution
      (return (Variables|Animations|GetExecutionMontages)))))

(fn GetStatCostforAction
  (bind _bp_statemanagercomponent (Variables|Default|GetBP_StateManagerComponent)
    (:then
      (return (.Value (Utilities|Map|Find (Variables|Stats|GetActionStatCost) (Default|GetCurrentAction _bp_statemanagercomponent)))))
    (:else
      (return 0.0))))

(fn GetDamage
  (bind _bp_statemanagercomponent (Variables|Default|GetBP_StateManagerComponent)
    (:then
      (return (* (Variables|Stats|GetDamage) (Math|Float|Clamp(Float) (.Value (Utilities|Map|Find (Variables|Stats|GetActionDamageMultiplier) (Default|GetCurrentAction _bp_statemanagercomponent))) 1.0 (.Value (Utilities|Map|Find (Variables|Stats|GetActionDamageMultiplier) (Default|GetCurrentAction _bp_statemanagercomponent)))))))
    (:else
      (return (Variables|Stats|GetDamage)))))

(fn ActivateCollision
  (params (CollisionPart :type E_CollisionPart%20Enum :default "NewEnumerator0"))
  (Default|ActivateCollision (Variables|Default|GetBP_MainCollisionComponent)))

(fn DeactivateCollision
  (params (CollisionPart :type E_CollisionPart%20Enum :default "NewEnumerator0"))
  (Default|DeactivateCollision (Variables|Default|GetBP_MainCollisionComponent)))

(fn ActivateTrailFX
  (if (Variables|FX|GetbEnableTrailFX?)
    (Effects|Particles|Trails|BeginTrails (Variables|Default|GetParticleSystem_Trail) "WeaponStartSocket" "WeaponEndSocket" "ETrailWidthMode_FromCentre" 1.0)))

(fn DeactivateTrailFX
  (if (Variables|FX|GetbEnableTrailFX?)
    (Effects|Particles|Trails|EndTrails (Variables|Default|GetParticleSystem_Trail))))

(fn ActivateDustFX
  (if (Variables|FX|GetbEnableDustFX?)
    (Effects|SpawnEmitterAttached (Variables|FX|GetDustFX) (CallFunction|GetItemMesh) "WeaponEndSocket" "0, 0, 0" "0, 0, 0" "1.000000,1.000000,1.000000" "KeepRelativeOffset" true "AutoRelease")))