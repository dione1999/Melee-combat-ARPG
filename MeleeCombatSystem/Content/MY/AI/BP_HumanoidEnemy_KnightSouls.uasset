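; Humanoid Knight Souls enemy Blueprint that adds music and a victory screen to its inherited enemy behavior.
; It listens to StateManagerComponent events, playing background music as a 2D sound when the Enter Combat action begins.
; When the Dead state begins, it waits briefly, then creates the WB_EnemyFelled widget and adds it to the viewport.
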(event OnCharacterStateBegin(StateManagerComponent)
  (params (CharacterState :type Gameplay%20Tag%20Structure))
  (|SwitchGameplayTag CharacterState
    (:Character.State.Dead
      (Utilities|FlowControl|Delay 1.5)
      (bind _returnvalue (UserInterface|CreateWidget "/Game/CombatSystem/UI/WB_EnemyFelled.WB_EnemyFelled_C"))
      (UserInterface|Viewport|AddtoViewport _returnvalue 0))))

(event OnCharacterActionBegin(StateManagerComponent)
  (params (Action :type Gameplay%20Tag%20Structure))
  (|SwitchGameplayTag Action
    (:Character.Action.Enter%20Combat
      (Audio|PlaySound2D (Variables|Default|GetBgm) 1.0 1.0 0.0 0 0))))

(event EventBeginPlay
  (|CallParentFunction))

(event Collision|EventActorBeginOverlap
  (params (OtherActor :type Actor%20Object%20Reference)))

(event EventTick
  (params (DeltaSeconds :type Float%20%28single-precision%29))
  (|CallParentFunction DeltaSeconds) ; This node is disabled and will not be called.\nDrag off pins to build functionality.
)

(fn ConstructionScript
  (|CallParentFunction))